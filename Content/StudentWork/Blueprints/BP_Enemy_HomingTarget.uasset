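; BP_Enemy_HomingTarget is an enemy variant whose attack fires a homing missile projectile.
; On Attack it spawns BP_EnemyProjectile_HomingMissile at the FireArrow component, aimed along the arrow's forward direction through a zero-degree cone, so without spread.
; When MyTarget is valid, it sets the missile's projectile movement homing target to that target's capsule component.
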(event `self.Attack`
  (bind _firearrow (`self.FireArrow`))
  (bind _mytarget (`self.MyTarget`))
  (bind _returnvalue (`|SpawnActorFromClass` "/Game/StudentWork/BP_EnemyProjectile_HomingMissile.BP_EnemyProjectile_HomingMissile_C" (`KismetMathLibrary.MakeTransform` (`SceneComponent.K2_GetComponentLocation` _firearrow) (`KismetMathLibrary.Conv_VectorToRotator` (`KismetMathLibrary.RandomUnitVectorInConeInDegrees` (`KismetMathLibrary.Conv_RotatorToVector` (`SceneComponent.K2_GetComponentRotation` _firearrow))))) "Undefined" "MultiplyWithRoot" null null))
  (`/Engine/EditorBlueprintResources/StandardMacros.IsValid` _mytarget
    (:`Is Valid`
      (set `ProjectileMovementComponent.HomingTargetComponent` (`Character.CapsuleComponent` _mytarget) (`/Game/StudentWork/BP_EnemyProjectile.ProjectileMovement` _returnvalue)))))

(fn `UserConstructionScript`
  (`parent.UserConstructionScript`))