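; Enemy Blueprint that fires an aimed projectile at its target when the Attack event runs.
; Attack checks that MyTarget is valid and not Dead, then spawns BP_EnemyProjectile at the FireArrow component's location.
; The projectile takes only the yaw of the look-at rotation toward the target, so shots aim horizontally.
; No movement or targeting logic is defined in these graphs, and the construction script only calls the parent's.
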(event `self.Attack`
  (bind _mytarget (`self.MyTarget`))
  (bind _returnvalue (`SceneComponent.K2_GetComponentLocation` (`self.FireArrow`)))
  (bind (_returnvalue_roll _returnvalue_pitch _returnvalue_yaw) (`KismetMathLibrary.BreakRotator` (`KismetMathLibrary.FindLookAtRotation` _returnvalue (`self.K2_GetActorLocation` _mytarget))))
  (`/Engine/EditorBlueprintResources/StandardMacros.IsValid` _mytarget
    (:`Is Valid`
      (if (not (`/Game/Blueprints/BP_PlayerCharacter.Dead` (`self.MyTarget`)))
        (`|SpawnActorFromClass` "/Game/StudentWork/Blueprints/Projectiles/BP_EnemyProjectile.BP_EnemyProjectile_C" (`KismetMathLibrary.MakeTransform` _returnvalue (`KismetMathLibrary.MakeRotator` 0.0 0.0 _returnvalue_yaw)) "Undefined" "MultiplyWithRoot" null null)))))

(fn `UserConstructionScript`
  (`parent.UserConstructionScript`))