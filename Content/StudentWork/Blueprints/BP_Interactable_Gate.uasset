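; Interactable gate Blueprint with two static meshes meant to slide apart when its Triggered event fires.
; Triggered plays the DoorOpen timeline, whose Distance track feeds GetMovement with opposite factors to set each mesh's world location.
; Each update starts from the mesh's current location rather than a stored origin.
; GetMovement contains only an unused X-axis Lerp, with no visible return value.
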(event `Event Triggered`
  (bind _staticmesh (`self.StaticMesh`))
  (bind _staticmesh2 (`self.StaticMesh2`))
  (bind (_direction _distance) (`Timeline|Door Open`)
    (:`Update`
      (bind _output_get (set `self.Distance` _distance))
      (`SceneComponent.K2_SetWorldLocation` _staticmesh (`self.GetMovement` _output_get 2.0 (`SceneComponent.K2_GetComponentLocation` _staticmesh)) false false)
      (`SceneComponent.K2_SetWorldLocation` _staticmesh2 (`self.GetMovement` (`self.Distance`) -2.0 (`SceneComponent.K2_GetComponentLocation` _staticmesh2)) false false))))

(fn `UserConstructionScript`)