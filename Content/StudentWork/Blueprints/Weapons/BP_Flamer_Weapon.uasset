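; Flamethrower weapon Blueprint for a tank, handling the visual and audio effects of firing.
; Started spawns the NS_Flamer effect attached to the tank's DirectionArrow and a non-auto-destroying shoot sound, storing both references.
; Completed deactivates the stored effect and stops the sound.
; The graph contains no damage or hit logic, and the construction script only calls its parent.
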(event `self.Started`
  (bind _returnvalue (`NiagaraFunctionLibrary.SpawnSystemAttached` "/Game/StudentWork/Particles/NS_Flamer.NS_Flamer" (`/Game/Blueprints/BP_PlayerCharacter.DirectionArrow` (`self.MyTank`)) "None" (0.0 0.0 0.0) (struct) "KeepRelativeOffset"))
  (set `self.FlamerSystem` _returnvalue)
  (bind _returnvalue_2 (`GameplayStatics.SpawnSoundAtLocation` (`self.ShootSound`) (0.0 0.0 0.0) (struct) 1.0 1.0 0.0 null null false))
  (set `self.FlamerAudio` _returnvalue_2))

(event `self.Completed`
  (`ActorComponent.Deactivate` (`self.FlamerSystem`))
  (`AudioComponent.Stop` (`self.FlamerAudio`)))

(fn `UserConstructionScript`
  (`parent.UserConstructionScript`))