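; Homing missile weapon that fires a Niagara missile effect from the tank's direction arrow at a BP_Enemy_HomingTarget actor.
; It takes the actor returned by GetActorOfClass and passes its capsule location to the effect once as the homing target.
; Damage is applied on a fixed timer rather than on impact, and a second timer clears the cooldown.
; The shoot sound node is unconnected.
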(event `self.Started`
  (bind _enemy (`self.Enemy`))
  (if (not (`self.Cooldown`))
    (bind _returnvalue (`NiagaraFunctionLibrary.SpawnSystemAttached` "/Game/StudentWork/Particles/NS_Homing_Missile.NS_Homing_Missile" (`/Game/Blueprints/BP_PlayerCharacter.DirectionArrow` (`self.MyTank`)) "None" (0.0 0.0 0.0) (struct) "KeepRelativeOffset" true))
    (set `self.Missiles` _returnvalue)
    (bind _returnvalue_2 (`GameplayStatics.GetActorOfClass` "/Game/StudentWork/Blueprints/Enemies/BP_Enemy_HomingTarget.BP_Enemy_HomingTarget_C"))
    (set `self.Enemy` _returnvalue_2)
    (`/Engine/EditorBlueprintResources/StandardMacros.IsValid` _enemy
      (:`Is Valid`
        (`ActorComponent.SetActive` (`self.Missiles`) true true)
        (`NiagaraComponent.SetVariableVec3` (`self.Missiles`) "HomingTarget" (`SceneComponent.K2_GetComponentLocation` (`Character.CapsuleComponent` _enemy)))
        (set `self.Cooldown` true)
        (`KismetSystemLibrary.K2_SetTimerDelegate` (delegate `End Cooldown`) (`self.Cooldown Time`))
        (`KismetSystemLibrary.K2_SetTimerDelegate` (delegate `Do Damage`) 1.2)))))

(event `Do Damage`
  (`GameplayStatics.ApplyDamage` (`self.Enemy`) 100.0))

(event `End Cooldown`
  (set `self.Cooldown` false))

(fn `UserConstructionScript`
  (`parent.UserConstructionScript`))