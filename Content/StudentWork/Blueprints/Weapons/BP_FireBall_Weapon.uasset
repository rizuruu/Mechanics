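; BP_FireBall_Weapon is a tank weapon that fires projectiles when triggered.
; Each shot spawns the WeaponProjectile class at the tank's DirectionArrow, aimed randomly within a narrow cone around the arrow's forward vector for spread.
; It also plays a projectile sound under a concurrency setting, and a short timer-cleared Cooldown flag limits the fire rate.
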(event `self.Triggered`
  (bind _directionarrow (`/Game/Blueprints/BP_PlayerCharacter.DirectionArrow` (`self.MyTank`)))
  (if (not (`self.Cooldown`))
    (bind _returnvalue (`|SpawnActorFromClass` (`self.Weapon Projectile`) (`KismetMathLibrary.MakeTransform` (`SceneComponent.K2_GetComponentLocation` _directionarrow) (`KismetMathLibrary.Conv_VectorToRotator` (`KismetMathLibrary.RandomUnitVectorInConeInDegrees` (`KismetMathLibrary.Conv_RotatorToVector` (`SceneComponent.K2_GetComponentRotation` _directionarrow)) 5.0))) "Undefined" "MultiplyWithRoot" null null))
    (`GameplayStatics.PlaySoundAtLocation` "/Game/StudentWork/Audio/MS_Projectile.MS_Projectile" (`self.K2_GetActorLocation`) (struct) 1.0 1.0 0.0 null "/Game/StudentWork/Audio/Projectile_Explosion_SC.Projectile_Explosion_SC" _returnvalue null)
    (set `self.Cooldown` true)
    (`KismetSystemLibrary.K2_SetTimerDelegate` (delegate `End Cooldown`) 0.4)))

(event `End Cooldown`
  (set `self.Cooldown` false))

(fn `UserConstructionScript`
  (`parent.UserConstructionScript`))