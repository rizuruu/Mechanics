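; BP_Laser_Weapon is a tank weapon that shoots fast projectiles when triggered.
; If off cooldown, the Triggered event spawns a BP_Fast_Projectile at the tank's direction arrow, matching its rotation.
; Each shot plays a sound with concurrency settings and a camera shake, then starts a short timer that clears the Cooldown flag to limit fire rate.
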(event `self.Triggered`
  (bind _directionarrow (`/Game/Blueprints/BP_PlayerCharacter.DirectionArrow` (`self.MyTank`)))
  (if (not (`self.Cooldown`))
    (bind _returnvalue (`|SpawnActorFromClass` "/Game/StudentWork/Blueprints/Projectiles/BP_Fast_Projectile.BP_Fast_Projectile_C" (`KismetMathLibrary.MakeTransform` (`SceneComponent.K2_GetComponentLocation` _directionarrow) (`SceneComponent.K2_GetComponentRotation` _directionarrow)) "Undefined" "MultiplyWithRoot" null null))
    (`GameplayStatics.PlaySoundAtLocation` (`self.ShootSound`) (`self.K2_GetActorLocation`) (struct) 1.0 1.0 0.0 null "/Game/StudentWork/Audio/Projectile_Explosion_SC.Projectile_Explosion_SC" _returnvalue null)
    (`self.Play Camera Shake`)
    (set `self.Cooldown` true)
    (`KismetSystemLibrary.K2_SetTimerDelegate` (delegate `End Cooldown`) 0.2)))

(event `End Cooldown`
  (set `self.Cooldown` false))

(fn `UserConstructionScript`
  (`parent.UserConstructionScript`))